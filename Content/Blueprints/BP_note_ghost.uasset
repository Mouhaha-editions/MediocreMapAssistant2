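; BP_note_ghost is a ghost version of a rhythm-game note, configured by Type, Direction, Line, Layer and Time.
; The construction script runs UpdateNote, which picks mesh and materials by Type, applies hardcoded red/blue colors to some types, and hides Arrow and Point.
; UpdateTransform derives X from Line, decoding thousand-scaled precise values, at fixed height.
; Layer and Time are returned by GetPos but don't affect placement.
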(event `Update Note`
  (bind _returnvalue (`KismetMathLibrary.Conv_LinearColorToVector` (struct :`R` 1.0 :`A` 1.0)))
  (bind _returnvalue_2 (`KismetMathLibrary.Conv_LinearColorToVector` (struct :`G` 0.33 :`B` 1.0 :`A` 1.0)))
  (bind _mesh (`self.Mesh`))
  (bind _arrow (`self.Arrow`))
  (bind _point (`self.Point`))
  (bind _point_2 (`self.Point`))
  (bind _arrow_2 (`self.Arrow`))
  (bind _mesh_2 (`self.Mesh`))
  (bind _mesh_3 (`self.Mesh`))
  (`|ExecutionSequence`
    (:`then_0`
      (switch `int` (`self.Type`)
        (:`0`
          (`StaticMeshComponent.SetStaticMesh` _mesh_3 "/Game/Meshes/SM_CubeNote.SM_CubeNote")
          (`PrimitiveComponent.SetMaterial` _mesh_3 0 "/Game/Materials/M_ghost_note_2.M_ghost_note_2")
          (`PrimitiveComponent.SetMaterial` _point 0 "/Game/Materials/M_Arrow_red.M_Arrow_red")
          (`PrimitiveComponent.SetMaterial` (`self.Arrow`) 0 "/Game/Materials/M_Arrow_red.M_Arrow_red")
          (if (== (`self.Direction`) 8) :!label _label
            (`SceneComponent.SetVisibility` _point_2 false false)
            (`SceneComponent.SetVisibility` _arrow_2 false false)
            (else
              (`SceneComponent.SetVisibility` _point_2 false false)
              (`SceneComponent.SetVisibility` _arrow_2 false false)))
          (`MeshComponent.SetVectorParameterValueOnMaterials` _mesh "Left" (/ _returnvalue 4))
          (`MeshComponent.SetVectorParameterValueOnMaterials` _mesh "Right" (/ _returnvalue_2 4))
          (`MeshComponent.SetVectorParameterValueOnMaterials` _arrow "Color_red" _returnvalue)
          (`MeshComponent.SetVectorParameterValueOnMaterials` (`self.Point`) "Color_red" _returnvalue)
          (`MeshComponent.SetVectorParameterValueOnMaterials` _arrow "Color_blue" _returnvalue_2)
          (`MeshComponent.SetVectorParameterValueOnMaterials` (`self.Point`) "Color_blue" _returnvalue_2)
          (`SceneComponent.K2_AddLocalTransform` _mesh_3 (`KismetMathLibrary.MakeTransform` (0.0 0.0 0.0) (struct) (1.0 1.0 1.0)) false false))
        (:`1`
          (`StaticMeshComponent.SetStaticMesh` _mesh_3 "/Game/Meshes/SM_CubeNote.SM_CubeNote")
          (`PrimitiveComponent.SetMaterial` _mesh_3 0 "/Game/Materials/M_ghost_note_blue.M_ghost_note_blue")
          (`PrimitiveComponent.SetMaterial` _point 0 "/Game/Materials/M_Arrow_blue.M_Arrow_blue")
          (`PrimitiveComponent.SetMaterial` (`self.Arrow`) 0 "/Game/Materials/M_Arrow_blue.M_Arrow_blue")
          (goto _label))
        (:`3`
          (`StaticMeshComponent.SetStaticMesh` _mesh_3 "/Game/Meshes/PK.PK")
          (`PrimitiveComponent.SetMaterial` _mesh_3 0 "/Game/Materials/M_ghost_note_3.M_ghost_note_3")
          (`SceneComponent.SetVisibility` (`self.Point`) false false)
          (`SceneComponent.SetVisibility` (`self.Arrow`) false false)
          (`SceneComponent.K2_AddLocalTransform` _mesh_3 (`KismetMathLibrary.MakeTransform` (0.0 0.0 0.0) (struct) (1.0 1.0 2.5)) false false))
        (:`4`
          (`StaticMeshComponent.SetStaticMesh` _mesh_2 "/Game/Meshes/SM_CubeNote.SM_CubeNote")
          (`PrimitiveComponent.SetMaterial` _mesh_2 0 "/Game/Materials/M_ghost_note_mag.M_ghost_note_mag")
          (`PrimitiveComponent.SetMaterial` (`self.Arrow`) 0 "/Game/Materials/M_Arrow_mag.M_Arrow_mag")
          (goto _label))
        (:`5`
          (`StaticMeshComponent.SetStaticMesh` _mesh_2 "/Game/Meshes/PK.PK")
          (`PrimitiveComponent.SetMaterial` _mesh_2 0 "/Game/Materials/M_ghost_note_green.M_ghost_note_green")
          (`PrimitiveComponent.SetMaterial` (`self.Arrow`) 0 "/Game/Materials/M_Arrow_green.M_Arrow_green")
          (goto _label))
        (:`6`
          (`StaticMeshComponent.SetStaticMesh` _mesh_2 "/Game/Meshes/PK.PK")
          (`PrimitiveComponent.SetMaterial` _mesh_2 0 "/Game/Materials/M_bomb_ghost.M_bomb_ghost")
          (`PrimitiveComponent.SetMaterial` (`self.Arrow`) 0 "/Game/Materials/M_Arrow_grey.M_Arrow_grey")
          (goto _label))))
    (:`then_1`
      (`self.UpdateTransform`))))

(event `UpdateTransform`
  (bind _line (`self.Line`))
  (bind _line_2 (`self.Line`))
  (bind _noteroot (`self.NoteRoot`))
  (`SceneComponent.K2_SetRelativeLocation` _noteroot (`KismetMathLibrary.MakeVector` (`KismetMathLibrary.SelectFloat` (- (* (/ (`KismetMathLibrary.Conv_IntToDouble` (`KismetMathLibrary.SelectInt` (- _line 1000) (+ _line 1000) (> _line 0))) 1000.0) 70.0) 105.0) (- (* (`self.Line`) 70.0) 105.0) (or (>= _line_2 1000) (<= _line_2 -1000))) 0.0 70.0) false false)
  (`SceneComponent.SetVisibility` _noteroot false false))

(fn `getPos`
  (returns (StructTimePos :type "/Game/Blueprints/VarTypes/StructTimePos Structure"))
  (return (make `/Game/Blueprints/VarTypes/StructTimePos` (`self.Time`) (`self.Line`) (`self.Layer`))))

(fn `UserConstructionScript`
  (`self.Update Note`))