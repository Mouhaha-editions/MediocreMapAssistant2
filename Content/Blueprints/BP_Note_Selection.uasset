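; BP_Note_Selection is a visual marker for a selected time range on a note track, apparently in a rhythm game.
; The construction script runs Init, which tints the start and end markers translucent cyan-blue, widens the layout in six-lane mode, then calls UpdateTransform.
; UpdateTransform converts Time and Duration through note separation into negative-Y offsets for both markers and stretches BottomCubes to span the range.
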(event `init`
  (bind _start (`self.Start`))
  (bind _start_2 (`self.Start`))
  (`MeshComponent.SetVectorParameterValueOnMaterials` _start "Emissive_Color" (0.0 1.0 2.0))
  (`MeshComponent.SetVectorParameterValueOnMaterials` (`self.EndMarker`) "Emissive_Color" (0.0 1.0 2.0))
  (`MeshComponent.SetScalarParameterValueOnMaterials` _start "Opacity" 0.1)
  (`MeshComponent.SetScalarParameterValueOnMaterials` (`self.EndMarker`) "Opacity" 0.1)
  (if (`/Game/Blueprints/BPFL_editor.Get6LaneMode`)
    (`SceneComponent.SetWorldScale3D` _start_2 (2.127 1.07 1.0))
    (`SceneComponent.SetWorldScale3D` (`self.EndMarker`) (2.127 1.07 1.0))
    (`SceneComponent.SetWorldScale3D` _start_2 (2.127 1.07 1.0))
    (`SceneComponent.SetWorldScale3D` (`self.EndMarker`) (2.127 1.07 1.0))
    (`SceneComponent.K2_SetWorldLocation` (`self.StaticMesh`) (-210.0 -5.0 0.0) false false)
    (`SceneComponent.K2_SetWorldLocation` (`self.Cube`) (210.0 -5.0 0.0) false false))
  (`self.UpdateTransform`))

(event `UpdateTransform`
  (bind _duration (`self.Duration`))
  (`SceneComponent.K2_SetRelativeLocation` (`self.Start`) (`KismetMathLibrary.MakeVector` 0.0 (* (* (`/Game/Blueprints/BPFL_editor.GetNoteSep`) (`self.Time`)) -1.0)) false false)
  (`SceneComponent.K2_SetRelativeLocation` (`self.BottomCubes`) (`KismetMathLibrary.MakeVector` 0.0 (* (* (`/Game/Blueprints/BPFL_editor.GetNoteSep`) (`self.Time`)) -1.0)) false false)
  (`SceneComponent.K2_SetRelativeLocation` (`self.EndMarker`) (`KismetMathLibrary.MakeVector` 0.0 (* (* (`/Game/Blueprints/BPFL_editor.GetNoteSep`) (+ (`self.Time`) _duration)) -1.0)) false false)
  (`SceneComponent.SetRelativeScale3D` (`self.BottomCubes`) (`KismetMathLibrary.MakeVector` 1.0 (* (`/Game/Blueprints/BPFL_editor.GetNoteSep`) _duration 0.1) 1.0)))

(fn `UserConstructionScript`
  (`self.init`))